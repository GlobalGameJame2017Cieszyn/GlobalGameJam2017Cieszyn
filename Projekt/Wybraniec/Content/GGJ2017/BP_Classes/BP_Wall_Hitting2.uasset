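; BP_Wall_Hitting2 is a moving wall hazard that kills the first-person player on contact.
; After a short startup delay, a looping timeline offsets the static mesh along relative Z from the location cached at BeginPlay, restarting each time it finishes.
; Any actor overlap is cast to FirstPersonCharacter, and a successful cast calls Die on that character.
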(event `self.ReceiveBeginPlay`
  (set `self.LOCAT` (`SceneComponent.RelativeLocation` (`self.StaticMesh`)))
  (`KismetSystemLibrary.Delay` 1.5)
  (bind (_direction _newtrack_0) (`Timeline|Timeline_0` :!label _label)
    (:`Update`
      (`SceneComponent.K2_SetRelativeLocation` (`self.StaticMesh`) (+ (`self.LOCAT`) (`KismetMathLibrary.MakeVector` 0.0 0.0 (.y _newtrack_0))) false false))
    (:`Finished`
      (`KismetSystemLibrary.Delay` 0.0)
      (goto _label :!via `PlayFromStart`))))

(event `self.ReceiveActorBeginOverlap`
  (params (OtherActor :type "Actor Object Reference"))
  (bind _asfirst_person_character (cast `/Game/FirstPersonBP/Blueprints/FirstPersonCharacter` OtherActor))
  (`/Game/FirstPersonBP/Blueprints/FirstPersonCharacter.Die` _asfirst_person_character))

(fn `UserConstructionScript`)