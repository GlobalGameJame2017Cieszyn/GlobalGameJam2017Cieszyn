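; Final power-up activator actor that the player triggers with the E key while overlapping it.
; Overlap begin and end toggle player input and a gate, so the key only works in range.
; BeginPlay binds to a CANBEDONE dispatcher that unlocks activation; E then calls the ActivateThePowerUp dispatcher.
; A Polish debug print stands in for an unfinished staff animation.
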(event `Key|E`
  (params (Key :type "Key Structure" :default "AnyKey"))
  (:`Pressed`
    (`/Engine/EditorBlueprintResources/StandardMacros.Gate` true :!label _label
      (:`Exit`
        (if (`self.CAN be donee`)
          (`KismetSystemLibrary.PrintString` "DO UZUPELNIENIA ANIMACJA KOSTURA KTORY COS ROBI Z TYM TYM")
          (`self.Activate the power up`))))))

(event `self.ReceiveActorBeginOverlap`
  (params (OtherActor :type "Actor Object Reference"))
  (`self.EnableInput` (`GameplayStatics.GetPlayerController` 0))
  (goto _label :!via `Open`))

(event `self.ReceiveActorEndOverlap`
  (params (OtherActor :type "Actor Object Reference"))
  (`self.DisableInput` (`GameplayStatics.GetPlayerController` 0))
  (goto _label :!via `Close`))

(event `self.ReceiveBeginPlay`
  (add `self.CAN BE DONE` (delegate `CAN BE DONE_Event`)))

(event `CAN BE DONE_Event`
  (set `self.CAN be donee` true))

(fn `UserConstructionScript`)