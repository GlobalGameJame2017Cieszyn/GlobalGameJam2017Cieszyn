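; Boss puzzle plate that lights its point light when shot, or when E is pressed inside its trigger box.
; A successful hit requires CantLightUp to be true despite its name, and a DoOnce limits it to one WasShot dispatch until reset.
; Bound events drive its state: CalledToLight shows the light and blocks hits, CantLightUp re-allows them, 10sUnlight clears the light and re-arms the DoOnce, and ResetAll does both latter.
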(event `Key|E`
  (params (Key :type "Key Structure" :default "AnyKey"))
  (:`Pressed`
    (`/Engine/EditorBlueprintResources/StandardMacros.Gate` true :!label _label
      (:`Exit`
        (if (`self.Cant light up`) :!label _label_2
          (`/Engine/EditorBlueprintResources/StandardMacros.DoOnce` false :!label _label_3
            (:`Completed`
              (`self.Was Shot`)
              (`SceneComponent.SetVisibility` (`self.PointLight`) true false))))))))

(event `self.Box.OnComponentBeginOverlap`
  (params (OverlappedComponent :type "PrimitiveComponent Object Reference") (OtherActor :type "Actor Object Reference") (OtherComp :type "PrimitiveComponent Object Reference") (OtherBodyIndex :type Integer) (bFromSweep :type Boolean) (SweepResult :type "HitResult Structure (by ref)"))
  (`self.EnableInput` (`GameplayStatics.GetPlayerController` 0))
  (goto _label :!via `Open`))

(event `self.Box.OnComponentEndOverlap`
  (params (OverlappedComponent :type "PrimitiveComponent Object Reference") (OtherActor :type "Actor Object Reference") (OtherComp :type "PrimitiveComponent Object Reference") (OtherBodyIndex :type Integer))
  (`self.DisableInput` (`GameplayStatics.GetPlayerController` 0))
  (goto _label :!via `Close`))

(event `PlayerShoot`
  (params (`Weapon Type` :type "/Game/FirstPersonBP/Blueprints/WeaponType Enum"))
  (goto _label_2))

(event `self.ReceiveBeginPlay`
  (`SceneComponent.SetVisibility` (`self.PointLight`) false false)
  (add `self.10sUnlight` (delegate `unl_Event`))
  (add `self.Reset all` (delegate `Reset all_Event`))
  (add `self.Can't Light Up` (delegate `Can't Light Up_Event`))
  (add `self.CalledToLight` (delegate `CalledToLight_Event`)))

(event `unl_Event`
  (`SceneComponent.SetVisibility` (`self.PointLight`) false false)
  (goto _label_3 :!via `Reset`))

(event `CalledToLight_Event`
  (`SceneComponent.SetVisibility` (`self.PointLight`) true false)
  (set `self.Cant light up` false))

(event `Reset all_Event`
  (set `self.Cant light up` true)
  (`SceneComponent.SetVisibility` (`self.PointLight`) false false)
  (goto _label_3 :!via `Reset`))

(event `Can't Light Up_Event`
  (set `self.Cant light up` true))

(fn `UserConstructionScript`)